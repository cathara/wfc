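; Wave Function Collapse tile that holds candidate data table rows and replaces its placeholder cube with a spawned tile actor.
; InitTile fills PossibilityArray with row names, which update functions prune by matching X1–X4 values, treating a required -1 as unconstrained.
; Waving spawns a random remaining candidate and stores its X values, while Collapse spawns without storing them.
; Debug prints trace comparisons and candidates, and ChangeColor tints the cube by type.
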(fn ConstructionScript)

(fn InitTile
  ;[1 1 1] reset the array
  (Utilities|Array|Clear (Variables|Default|Getpossibility_array))
  ;[1 1 1] get all the names
  (bind _outrownames (DataTable|GetDataTableRowNames (Variables|Default|Getwfc_tile_datatable)))
  ;[1 1 1] create possibility array with all the name
  (for _array_element _outrownames
    (Utilities|Array|Add (Variables|Default|Getpossibility_array) _array_element)
    (Development|PrintString (Utilities|String|ToString(Name) _array_element))
    (bind _returnvalue (Utilities|GetDataTableRow "/Game/wfc/tile_data_table/wfc_tile_v1.wfc_tile_v1" _array_element)
      (:then
        (Development|PrintString (Utilities|String|Append "DATA TABLE ROW EQUAL : " (Utilities|String|ToString(Integer) (.x1 _returnvalue)) "/" (Utilities|String|ToString(Integer) (.x2 _returnvalue)) "/" (Utilities|String|ToString(Integer) (.x3 _returnvalue)) "/" (Utilities|String|ToString(Integer) (.x4 _returnvalue))))))))

(fn GetX1
  (return (Variables|Default|GetX1)))

(fn GetX2
  (return (Variables|Default|GetX2)))

(fn GetX3
  (return (Variables|Default|GetX3)))

(fn GetX4
  (return (Variables|Default|GetX4)))

(fn UpdatePosibilityArray
  ;[1 1 1] iterate over each position of the possibility array and checking if the position exist
  (for _array_element (Variables|Default|Getpossibility_array)
    (bind _returnvalue (Class|DataTableFunctionLibrary|DoesDataTableRowExist "/Game/wfc/tile_data_table/wfc_tile_v1.wfc_tile_v1" _array_element))
    (if _returnvalue
      ;[1 1 1] ye wtf
      (bind _returnvalue_2 (Utilities|GetDataTableRow "/Game/wfc/tile_data_table/wfc_tile_v1.wfc_tile_v1" _array_element)
        (:then
          (CallFunction|CheckValues (Variables|Default|GetX1) (.x1 _returnvalue_2) _array_element)
          (CallFunction|CheckValues (Variables|Default|GetX2) (.x2 _returnvalue_2) _array_element)
          (CallFunction|CheckValues (Variables|Default|GetX3) (.x3 _returnvalue_2) _array_element)
          (CallFunction|CheckValues (Variables|Default|GetX4) (.x4 _returnvalue_2) _array_element))))))

(fn CheckValues
  (params (current_x :type Integer) (row_x :type Integer) (current_name :type Name))
  (if (!= -1 current_x)
    (if (!= current_x row_x)
      (Utilities|Array|RemoveItem (Variables|Default|Getpossibility_array) current_name))))

(fn Collapse
  (bind _possibility_array (Variables|Default|Getpossibility_array))
  (bind _cube (Variables|Default|GetCube))
  (bind _possibility_array_2 (Variables|Default|Getpossibility_array))
  (bind _cube_2 (Variables|Default|GetCube))
  (bind _returnvalue (Utilities|Array|Length _possibility_array))
  (if (== _returnvalue 1)
    (Components|DestroyComponent (Variables|Default|GetCube))
    (bind _returnvalue_2 (Utilities|GetDataTableRow "/Game/wfc/tile_data_table/wfc_tile_v1.wfc_tile_v1" (Utilities|Array|Get(acopy) _possibility_array_2 (Utilities|Array|LastIndex _possibility_array_2)))
      (:then
        (Game|SpawnActorfromClass (.tile_actor _returnvalue_2) (Math|Transform|MakeTransform (Transformation|GetWorldLocation _cube_2) "0, 0, 0" "1.000000,1.000000,1.000000") "Undefined" "MultiplyWithRoot" 0 0)
        (Components|DestroyComponent _cube_2)))
    (else
      (bind _returnvalue_3 (Utilities|GetDataTableRow "/Game/wfc/tile_data_table/wfc_tile_v1.wfc_tile_v1" (Utilities|Array|Get(acopy) (Variables|Default|Getpossibility_array) (Math|Random|RandomInteger _returnvalue)))
        (:then
          (bind _returnvalue_4 (Game|SpawnActorfromClass (.tile_actor _returnvalue_3) (Math|Transform|MakeTransform (Transformation|GetWorldLocation _cube) "0, 0, 0" "1.000000,1.000000,1.000000") "Undefined" "MultiplyWithRoot" 0 0))
          (Components|DestroyComponent _cube)
          (return _returnvalue_4))))))

(fn ChangeColor
  (params (tile%20type :type Integer))
  (switch int tile%20type
    (:1
      (Rendering|Material|SetVectorParameterValueonMaterials (Variables|Default|GetCube) "constant" "1.000000,1.000000,1.000000"))
    (:2
      (Rendering|Material|SetVectorParameterValueonMaterials (Variables|Default|GetCube) "constant" "1.000000,0.000000,1.000000"))
    (:3
      (Rendering|Material|SetVectorParameterValueonMaterials (Variables|Default|GetCube) "constant" "1.000000,1.000000,0.000000"))
    (:4
      (Rendering|Material|SetVectorParameterValueonMaterials (Variables|Default|GetCube) "constant" "0.000000,0.000000,0.000000"))))

(fn UpdateTilePosX1
  (params (X1 :type Integer))
  (bind _possibility_array (Variables|Default|Getpossibility_array))
  (Utilities|Array|Clear (Variables|Default|Getremove_array))
  (for _array_element (Variables|Default|Getpossibility_array)
    (bind _returnvalue (Utilities|GetDataTableRow "/Game/wfc/tile_data_table/wfc_tile_v1.wfc_tile_v1" _array_element)
      (:then
        (Development|PrintString (Utilities|String|Append (Utilities|String|ToString(Integer) (.x1 _returnvalue)) "-" (Utilities|String|ToString(Integer) (.x2 _returnvalue)) "-" (Utilities|String|ToString(Integer) (.x3 _returnvalue)) "-" (Utilities|String|ToString(Integer) (.x4 _returnvalue)))))))
  (for _array_element_2 _possibility_array
    (bind _returnvalue_2 (Utilities|GetDataTableRow "/Game/wfc/tile_data_table/wfc_tile_v1.wfc_tile_v1" _array_element_2)
      (:then
        (bind _remove (CallFunction|CompareX (.x1 _returnvalue_2) X1))
        (if _remove
          (Utilities|Array|Add (Variables|Default|Getremove_array) _array_element_2)))))
  (for _array_element_3 (Variables|Default|Getremove_array)
    (bind _returnvalue_3 (Class|DataTableFunctionLibrary|DoesDataTableRowExist "/Game/wfc/tile_data_table/wfc_tile_v1.wfc_tile_v1" _array_element_3))
    (if _returnvalue_3
      (Utilities|Array|RemoveItem (Variables|Default|Getpossibility_array) _array_element_3)))
  (for _array_element_4 _possibility_array
    (bind _returnvalue_4 (Utilities|GetDataTableRow "/Game/wfc/tile_data_table/wfc_tile_v1.wfc_tile_v1" _array_element_4)
      (:then
        (Development|PrintString (Utilities|String|Append (Utilities|String|ToString(Integer) (.x1 _returnvalue_4)) "   " (Utilities|String|ToString(Integer) (.x2 _returnvalue_4)) "   " (Utilities|String|ToString(Integer) (.x3 _returnvalue_4)) "   " (Utilities|String|ToString(Integer) (.x4 _returnvalue_4))))))))

(fn UpdateTilePosX2
  (params (X2 :type Integer))
  (bind _possibility_array (Variables|Default|Getpossibility_array))
  (Utilities|Array|Clear (Variables|Default|Getremove_array))
  (for _array_element _possibility_array
    (bind _returnvalue (Utilities|GetDataTableRow "/Game/wfc/tile_data_table/wfc_tile_v1.wfc_tile_v1" _array_element)
      (:then
        (bind _remove (CallFunction|CompareX (.x2 _returnvalue) X2))
        (if _remove
          (Utilities|Array|Add (Variables|Default|Getremove_array) _array_element)))))
  (for _array_element_2 (Variables|Default|Getremove_array)
    (bind _returnvalue_2 (Class|DataTableFunctionLibrary|DoesDataTableRowExist "/Game/wfc/tile_data_table/wfc_tile_v1.wfc_tile_v1" _array_element_2))
    (if _returnvalue_2
      (Utilities|Array|RemoveItem (Variables|Default|Getpossibility_array) _array_element_2)))
  (for _array_element_3 _possibility_array
    (bind _returnvalue_3 (Utilities|GetDataTableRow "/Game/wfc/tile_data_table/wfc_tile_v1.wfc_tile_v1" _array_element_3)
      (:then
        (Development|PrintString (Utilities|String|Append (Utilities|String|ToString(Integer) (.x1 _returnvalue_3)) "   " (Utilities|String|ToString(Integer) (.x2 _returnvalue_3)) "   " (Utilities|String|ToString(Integer) (.x3 _returnvalue_3)) "   " (Utilities|String|ToString(Integer) (.x4 _returnvalue_3))))))))

(fn UpdateTilePosX3
  (params (X3 :type Integer))
  (bind _possibility_array (Variables|Default|Getpossibility_array))
  (Utilities|Array|Clear (Variables|Default|Getremove_array))
  (for _array_element _possibility_array
    (bind _returnvalue (Utilities|GetDataTableRow "/Game/wfc/tile_data_table/wfc_tile_v1.wfc_tile_v1" _array_element)
      (:then
        (bind _remove (CallFunction|CompareX (.x3 _returnvalue) X3))
        (if _remove
          (Utilities|Array|Add (Variables|Default|Getremove_array) _array_element)))))
  (for _array_element_2 (Variables|Default|Getremove_array)
    (bind _returnvalue_2 (Class|DataTableFunctionLibrary|DoesDataTableRowExist "/Game/wfc/tile_data_table/wfc_tile_v1.wfc_tile_v1" _array_element_2))
    (if _returnvalue_2
      (Utilities|Array|RemoveItem (Variables|Default|Getpossibility_array) _array_element_2)))
  (for _array_element_3 _possibility_array
    (bind _returnvalue_3 (Utilities|GetDataTableRow "/Game/wfc/tile_data_table/wfc_tile_v1.wfc_tile_v1" _array_element_3)
      (:then
        (Development|PrintString (Utilities|String|Append (Utilities|String|ToString(Integer) (.x1 _returnvalue_3)) "   " (Utilities|String|ToString(Integer) (.x2 _returnvalue_3)) "   " (Utilities|String|ToString(Integer) (.x3 _returnvalue_3)) "   " (Utilities|String|ToString(Integer) (.x4 _returnvalue_3))))))))

(fn UpdateTilePosX4
  (params (x4 :type Integer))
  (bind _possibility_array (Variables|Default|Getpossibility_array))
  (Utilities|Array|Clear (Variables|Default|Getremove_array))
  (for _array_element _possibility_array
    (bind _returnvalue (Utilities|GetDataTableRow "/Game/wfc/tile_data_table/wfc_tile_v1.wfc_tile_v1" _array_element)
      (:then
        (bind _remove (CallFunction|CompareX (.x4 _returnvalue) x4))
        (if _remove
          (Utilities|Array|Add (Variables|Default|Getremove_array) _array_element)))))
  (for _array_element_2 (Variables|Default|Getremove_array)
    (bind _returnvalue_2 (Class|DataTableFunctionLibrary|DoesDataTableRowExist "/Game/wfc/tile_data_table/wfc_tile_v1.wfc_tile_v1" _array_element_2))
    (if _returnvalue_2
      (Utilities|Array|RemoveItem (Variables|Default|Getpossibility_array) _array_element_2)))
  (for _array_element_3 _possibility_array
    (bind _returnvalue_3 (Utilities|GetDataTableRow "/Game/wfc/tile_data_table/wfc_tile_v1.wfc_tile_v1" _array_element_3)
      (:then
        (Development|PrintString (Utilities|String|Append (Utilities|String|ToString(Integer) (.x1 _returnvalue_3)) "   " (Utilities|String|ToString(Integer) (.x2 _returnvalue_3)) "   " (Utilities|String|ToString(Integer) (.x3 _returnvalue_3)) "   " (Utilities|String|ToString(Integer) (.x4 _returnvalue_3))))))))

(fn CompareX
  (params (tx :type Integer) (x :type Integer))
  (Development|PrintString (Utilities|String|Append "comparing" (Utilities|String|ToString(Integer) tx) " and " (Utilities|String|ToString(Integer) x)))
  (Utilities|FlowControl|Sequence
    (:then_0
      (if (== tx x)
        (Variables|Default|Setremove false)
        (else
          (Variables|Default|Setremove true))))
    (:then_1
      (if (== x -1)
        (Variables|Default|Setremove false)))
    (:then_2
      (return (Variables|Default|Getremove)))))

(fn Waving
  (bind _cube (Variables|Default|GetCube))
  (bind _returnvalue (Utilities|GetDataTableRow "/Game/wfc/tile_data_table/wfc_tile_v1.wfc_tile_v1" (.OutItem (Utilities|Array|Random (Variables|Default|Getpossibility_array))))
    (:then
      (Variables|Default|SetX1 (.x1 _returnvalue))
      (Variables|Default|SetX2 (.x2 _returnvalue))
      (Variables|Default|SetX3 (.x3 _returnvalue))
      (Variables|Default|SetX4 (.x4 _returnvalue))
      (Development|PrintString (Utilities|String|Append "tile collapsed to :" (Utilities|String|ToString(Integer) (.x1 _returnvalue)) "-" (Utilities|String|ToString(Integer) (.x2 _returnvalue)) "-" (Utilities|String|ToString(Integer) (.x3 _returnvalue)) "-" (Utilities|String|ToString(Integer) (.x4 _returnvalue))))
      (bind _returnvalue_2 (Game|SpawnActorfromClass (.tile_actor _returnvalue) (Transformation|GetWorldTransform _cube) "Undefined" "MultiplyWithRoot" 0 0))
      (Components|DestroyComponent _cube)
      (return _returnvalue_2))))